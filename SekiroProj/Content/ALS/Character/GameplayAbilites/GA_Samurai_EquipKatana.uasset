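; Gameplay ability that equips the player samurai's katana.
; It plays an equip montage and waits for a gameplay event to snap the carried weapon to the right-hand katana socket and mark it as equipped.
; HadleEquipWeapon then uses the weapon's data to add its input mapping context, grant its abilities, and store the granted spec handles on the weapon.
; The ability ends when the montage completes, blends out, or is interrupted or cancelled.
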(event `self.K2_ActivateAbility`
  (`AbilityTask_PlayMontageAndWait.CreatePlayMontageAndWaitProxy` "None" "/Game/ALS/Animations/Katana/Equip/AM_MM_Katana_Equip.AM_MM_Katana_Equip"
    (:`then`
      (`AbilityTask_WaitGameplayEvent.WaitGameplayEvent` (struct :`TagName` "Player.Event.Equip.Katana") null
        (:`EventReceived`
          (`Actor.K2_AttachToComponent` (`PawnCombatComponent.GetCharacterCarriedWeaponByTag` (`self.GetPlayerCombatComponentFromActorInfo`) (struct :`TagName` "Player.Weapon.Katana")) (`self.GetOwningComponentFromActorInfo`) "katana_r" "SnapToTarget" "KeepRelative" "KeepRelative" true)
          (`self.HadleEquipWeapon` (`PlayerCombatComponent.GetPlayerCarriedWeaponByTag` (`self.GetPlayerCombatComponentFromActorInfo`) (struct :`TagName` "Player.Weapon.Katana")))
          (set `PawnCombatComponent.CurrentEquippedWeaponTag` (struct :`TagName` "Player.Weapon.Katana") (`self.GetPlayerCombatComponentFromActorInfo`)))))
    (:`OnCompleted`
      (`self.K2_EndAbility` :!label _label))
    (:`OnBlendOut`
      (goto _label))
    (:`OnInterrupted`
      (goto _label))
    (:`OnCancelled`
      (goto _label))))

(fn `HadleEquipWeapon`
  (params (`In Weapon to Equip` :type "SekiroWeaponKatana Object Reference"))
  (locals (CachedPlayerWeaponData :type "SekiroWeaponData Structure"))
  (set `local.CachedPlayerWeaponData` (`SekiroWeaponKatana.SamuraiWeaponData` `In Weapon to Equip`))
  (`|ExecutionSequence`
    (:`then_1`
      (`EnhancedInputSubsystemInterface.AddMappingContext` (pcsubsystem `EnhancedInputLocalPlayerSubsystem` (`self.GetPlayerControllerFromActorInfo`)) (`.WeaponInputMappingContext` (break `SekiroWeaponData` (`local.CachedPlayerWeaponData`))) 1 (struct)))
    (:`then_2`
      (bind _outgrantedabilityspechandles (`SekiroAbilitySystemComponent.GrantSekiroWeaponAbilities` (`self.GetSekiroASCFromActorInfo`) (`.DefaultWeaponAbilities` (break `SekiroWeaponData` (`local.CachedPlayerWeaponData`))) (`self.GetAbilityLevel`)))
      (`SekiroWeaponKatana.AssignGrantedAbilitySpecHandles` (`local.In Weapon to Equip`) _outgrantedabilityspechandles))))
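; Samurai master Gameplay Ability for weapon attacks that chains a montage-based melee combo across repeated activations.
; Each activation clears the pending reset timer and plays the montage mapped to the current combo count from its "Attack_Hit" section.
; The count advances as the montage starts, wrapping to the first attack after the last map entry.
; Montage completion, blend out, interruption or cancellation ends the ability and starts a short combo-reset timer.
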(event `self.K2_ActivateAbility`
  (`KismetSystemLibrary.K2_ClearAndInvalidateTimerHandle` (`self.ComboCountResetTimerHandle`))
  (set `self.Used Combo Count` (`self.Current Attack Combo Count`))
  (`AbilityTask_PlayMontageAndWait.CreatePlayMontageAndWaitProxy` "None" (`BlueprintMapLibrary.Map_Find` (`self.AttackMontagesMap`) (`self.Current Attack Combo Count`)) 1.0 "Attack_Hit" true 1.0 0.0 true
    (:`then`
      (`|ExecutionSequence`
        (:`then_2`
          (if (`self.CheckCurrentAttackComboCount`)
            (`self.ResetAttackComboCount`)
            (else
              (if (`self.CheckCurrentAttackComboCountMinus`)
                _
                (else
                  _))
              (`/Engine/EditorBlueprintResources/StandardMacros.IncrementInt` (`self.Current Attack Combo Count`)))))))
    (:`OnCompleted`
      (`self.K2_EndAbility` :!label _label)
      (bind _returnvalue (`KismetSystemLibrary.K2_SetTimerDelegate` (delegate `ResetAttackComboCount`) 0.3))
      (set `self.ComboCountResetTimerHandle` _returnvalue))
    (:`OnBlendOut`
      (goto _label))
    (:`OnInterrupted`
      (goto _label))
    (:`OnCancelled`
      (goto _label))))

(event `ResetAttackComboCount`
  (set `self.Current Attack Combo Count` 1))

(fn `CheckCurrentAttackComboCount`
  (returns (`Return Value` :type Boolean))
  (return (== (`self.Current Attack Combo Count`) (`BlueprintMapLibrary.Map_Length` (`self.AttackMontagesMap`)))))

(fn `CheckCurrentAttackComboCountMinus`
  (returns (`Return Value` :type Boolean))
  (return (== (`self.Current Attack Combo Count`) (- (`BlueprintMapLibrary.Map_Length` (`self.AttackMontagesMap`)) 1))))
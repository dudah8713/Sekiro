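; Gameplay ability for the samurai katana combo attack that tracks the input timing window between combo hits.
; When the montage starts, it waits on Combo_Start and Combo_End gameplay events to open and close the window.
; If no input arrived at the right time when the window closes, it resets the combo count to one and ends the ability.
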(event `self.MontageStarted`
  (`AbilityTask_WaitGameplayEvent.WaitGameplayEvent` (struct :`TagName` "InputTag.MeleeAttack.Katana.Combo_Start") null
    (:`then`
      (`AbilityTask_WaitGameplayEvent.WaitGameplayEvent` (struct :`TagName` "InputTag.MeleeAttack.Katana.Combo_End") null
        (:`then`
          (`KismetSystemLibrary.PrintString` (`KismetStringLibrary.Conv_IntToString` (`self.Current Attack Combo Count`))))
        (:`EventReceived`
          (set `self.IsWithinComboWindow` false)
          (if (not (`self.ReceivedInputAtRightTime`))
            (set `self.Current Attack Combo Count` 1)
            (`self.K2_EndAbility`)))))
    (:`EventReceived`
      (set `self.IsWithinComboWindow` true))))
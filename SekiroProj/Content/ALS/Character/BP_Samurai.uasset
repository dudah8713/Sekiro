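; Player-controlled samurai character with Enhanced Input for look, move, jump, run, crouch and weapon switching, using layered locomotion animation.
; Run and crouch inputs change the gait via UpdateGate, which applies DT_KatanaGate movement rows chosen by gait and weapon.
; The anim instance receives gait, weapon and traced ground distance, while weapons link anim class layers.
; Katana layers link at BeginPlay, but katana switch and equip montage are unwired.
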(event `self.ReceiveTick`
  (params (DeltaSeconds :type "Float (single-precision)"))
  (`|ExecutionSequence`
    (:`then_0`
      (bind (_outhit _returnvalue) (`KismetSystemLibrary.SphereTraceSingle` (- (`self.K2_GetActorLocation`) (`KismetMathLibrary.MakeVector` 0.0 0.0 (`CapsuleComponent.CapsuleHalfHeight` (`self.CapsuleComponent`)))) (- (`self.K2_GetActorLocation`) (0.0 0.0 1000.0)) 5.0 "TraceTypeQuery1"))
      (if _returnvalue
        (message `/Game/ALS/Interface/BPI_AnimationInterface.RecieveGroundDistance` (`SkeletalMeshComponent.GetAnimInstance` (`self.Mesh`)) (`.Distance` (`GameplayStatics.BreakHitResult` _outhit)))))))

(event `self.ReceiveBeginPlay`
  (bind _asplayer_controller (cast `PlayerController` (`self.GetController`)))
  (message `EnhancedInputSubsystemInterface.AddMappingContext` (pcsubsystem `EnhancedInputLocalPlayerSubsystem` _asplayer_controller) "/Game/ALS/Inputs/IMC_ALS.IMC_ALS" 0 (struct))
  (`SkeletalMeshComponent.LinkAnimClassLayers` (`self.Mesh`) "/Game/ALS/AnimationBlueprints/APB_Katana.APB_Katana_C")
  (`self.UpdateGate` "NewEnumerator0"))

(event `EnhancedInput|/Game/ALS/Inputs/InputActions/IA_Look`
  (params (ActionValue :type "Vector2D Structure") (ElapsedSeconds :type "Float (double-precision)") (TriggeredSeconds :type "Float (double-precision)") (InputAction :type "InputAction Object Reference" :default "/Game/ALS/Inputs/InputActions/IA_Look.IA_Look"))
  (bind (_x _y) (`KismetMathLibrary.BreakVector2D` ActionValue))
  (:`Triggered`
    (`self.AddControllerYawInput` _x)
    ; Spring Arm의 Use Pawn Control Rotation Check
    (`self.AddControllerPitchInput` _y)))

(event `EnhancedInput|/Game/ALS/Inputs/InputActions/IA_Move`
  (params (ActionValue :type "Vector2D Structure") (ElapsedSeconds :type "Float (double-precision)") (TriggeredSeconds :type "Float (double-precision)") (InputAction :type "InputAction Object Reference" :default "/Game/ALS/Inputs/InputActions/IA_Move.IA_Move"))
  (bind (_x _y) (`KismetMathLibrary.BreakVector2D` ActionValue))
  (bind (_returnvalue_roll _returnvalue_pitch _returnvalue_yaw) (`KismetMathLibrary.BreakRotator` (`self.GetControlRotation`)))
  (bind (_returnvalue_roll_2 _returnvalue_pitch_2 _returnvalue_yaw_2) (`KismetMathLibrary.BreakRotator` (`self.GetControlRotation`)))
  (:`Triggered`
    ; 좌, 우 이동
    (`self.AddMovementInput` (`KismetMathLibrary.GetRightVector` (`KismetMathLibrary.MakeRotator` _returnvalue_roll_2 0.0 _returnvalue_yaw_2)) _x)
    ; 앞, 뒤 이동
    (`self.AddMovementInput` (`KismetMathLibrary.GetForwardVector` (`KismetMathLibrary.MakeRotator` 0.0 0.0 _returnvalue_yaw)) _y)
    ; 뒤를 향할 때의 가속도 값 수정, start fwd 짧아서
    (if (`self.CheckDirection`)
      (set `CharacterMovementComponent.MaxAcceleration` 1000.0 (`self.CharacterMovement`)))))

(event `EnhancedInput|/Game/ALS/Inputs/InputActions/IA_Look`
  (params (ActionValue :type "Vector2D Structure") (ElapsedSeconds :type "Float (double-precision)") (TriggeredSeconds :type "Float (double-precision)") (InputAction :type "InputAction Object Reference" :default "/Game/ALS/Inputs/InputActions/IA_Look.IA_Look"))
  (:`Triggered`
    (`self.AddControllerYawInput` (`KismetMathLibrary.BreakVector2D` ActionValue))))

(event `EnhancedInput|/Game/ALS/Inputs/InputActions/IA_SwitchWeapon`
  (params (ActionValue :type "Float (double-precision)") (ElapsedSeconds :type "Float (double-precision)") (TriggeredSeconds :type "Float (double-precision)") (InputAction :type "InputAction Object Reference" :default "/Game/ALS/Inputs/InputActions/IA_SwitchWeapon.IA_SwitchWeapon"))
  (:`Triggered`
    (switch `int` (`KismetMathLibrary.FTrunc` ActionValue)
      (:`1`
        (set `self.EquipedWeapon` "NewEnumerator0")
        (`SkeletalMeshComponent.LinkAnimClassLayers` (`self.Mesh`) "/Game/ALS/AnimationBlueprints/ABP_UnArmed.ABP_UnArmed_C")
        (message `/Game/ALS/Interface/BPI_AnimationInterface.RecieveEquipedWeapon` (`SkeletalMeshComponent.GetAnimInstance` (`self.Mesh`)) (`self.EquipedWeapon`)))
      (:`3`
        (set `self.EquipedWeapon` "NewEnumerator2")))))

(event `EnhancedInput|/Game/ALS/Inputs/InputActions/IA_Run`
  (params (ActionValue :type Boolean) (ElapsedSeconds :type "Float (double-precision)") (TriggeredSeconds :type "Float (double-precision)") (InputAction :type "InputAction Object Reference" :default "/Game/ALS/Inputs/InputActions/IA_Run.IA_Run"))
  (bind _currentgate (`self.CurrentGate`))
  (:`Started`
    (switch `/Game/ALS/Enums/E_Gate` _currentgate
      (:`NewEnumerator0`
        (`self.UpdateGate` "NewEnumerator1" :!label _label))
      (:`NewEnumerator1`
        (goto _label))
      (:`NewEnumerator2`
        (`self.UpdateGate` "NewEnumerator3" :!label _label_2))
      (:`NewEnumerator3`
        (goto _label_2))))
  (:`Completed`
    (switch `/Game/ALS/Enums/E_Gate` _currentgate
      (:`NewEnumerator0`
        (`self.UpdateGate` "NewEnumerator0" :!label _label_3))
      (:`NewEnumerator1`
        (goto _label_3))
      (:`NewEnumerator2`
        (`self.UpdateGate` "NewEnumerator2" :!label _label_4))
      (:`NewEnumerator3`
        (goto _label_4)))))

(event `EnhancedInput|/Game/ALS/Inputs/InputActions/IA_Crouch`
  (params (ActionValue :type Boolean) (ElapsedSeconds :type "Float (double-precision)") (TriggeredSeconds :type "Float (double-precision)") (InputAction :type "InputAction Object Reference" :default "/Game/ALS/Inputs/InputActions/IA_Crouch.IA_Crouch"))
  (:`Started`
    (switch `/Game/ALS/Enums/E_Gate` (`self.CurrentGate`)
      (:`NewEnumerator0`
        (`self.UpdateGate` "NewEnumerator2")
        (`self.Crouch` :!label _label_5))
      (:`NewEnumerator1`
        (`self.UpdateGate` "NewEnumerator3")
        (goto _label_5))
      (:`NewEnumerator2`
        (`self.UpdateGate` "NewEnumerator0")
        (`self.UnCrouch` :!label _label_6))
      (:`NewEnumerator3`
        (`self.UpdateGate` "NewEnumerator1")
        (goto _label_6)))))

(event `EnhancedInput|/Game/ALS/Inputs/InputActions/IA_Jump`
  (params (ActionValue :type Boolean) (ElapsedSeconds :type "Float (double-precision)") (TriggeredSeconds :type "Float (double-precision)") (InputAction :type "InputAction Object Reference" :default "/Game/ALS/Inputs/InputActions/IA_Jump.IA_Jump"))
  (:`Started`
    (`self.Jump`))
  (:`Completed`
    (`self.StopJumping`)))

(event `EnhancedInput|/Game/ALS/Inputs/InputActions/IA_Aim`
  (params (ActionValue :type Boolean) (ElapsedSeconds :type "Float (double-precision)") (TriggeredSeconds :type "Float (double-precision)") (InputAction :type "InputAction Object Reference" :default "/Game/ALS/Inputs/InputActions/IA_Aim.IA_Aim")))

(fn `CheckDirection`
  (returns (ReturnValue :type Boolean))
  (return (< (`KismetMathLibrary.Dot_VectorVector` (`KismetMathLibrary.Normal` (`CharacterMovementComponent.GetLastUpdateVelocity` (`self.CharacterMovement`))) (`self.GetActorForwardVector`)) -0.5)))

(fn `UpdateGate`
  (params (Gate :type "/Game/ALS/Enums/E_Gate Enum" :default "NewEnumerator0"))
  (set `self.CurrentGate` Gate)
  (message `/Game/ALS/Interface/BPI_AnimationInterface.RecieveCurrentGate` (`SkeletalMeshComponent.GetAnimInstance` (`self.Mesh`)) (`local.Gate`))
  (switch `/Game/ALS/Enums/E_Gate` (`self.CurrentGate`)
    (:`NewEnumerator0`
      (switch `/Game/ALS/Enums/E_Weapons` (`self.EquipedWeapon`)
        (:`NewEnumerator0`
          (bind _returnvalue (`|GetDataTableRow` "/Game/ALS/DataTables/DT_KatanaGate.DT_KatanaGate" "UnarmedWalk")
            (:`then`
              (`self.SetGateSettings` _returnvalue))))
        (:`NewEnumerator1`
          (bind _returnvalue_2 (`|GetDataTableRow` "/Game/ALS/DataTables/DT_KatanaGate.DT_KatanaGate" "KatanaWalk")
            (:`then`
              (`self.SetGateSettings` _returnvalue_2))))))
    (:`NewEnumerator1`
      (switch `/Game/ALS/Enums/E_Weapons` (`self.EquipedWeapon`)
        (:`NewEnumerator0`
          (bind _returnvalue_3 (`|GetDataTableRow` "/Game/ALS/DataTables/DT_KatanaGate.DT_KatanaGate" "UnarmedJog")
            (:`then`
              (`self.SetGateSettings` _returnvalue_3))))
        (:`NewEnumerator1`
          (bind _returnvalue_4 (`|GetDataTableRow` "/Game/ALS/DataTables/DT_KatanaGate.DT_KatanaGate" "KatanaJog")
            (:`then`
              (`self.SetGateSettings` _returnvalue_4))))))
    (:`NewEnumerator2`
      (switch `/Game/ALS/Enums/E_Weapons` (`self.EquipedWeapon`)
        (:`NewEnumerator0`
          (bind _returnvalue_5 (`|GetDataTableRow` "/Game/ALS/DataTables/DT_KatanaGate.DT_KatanaGate" "UnarmedCrouch")
            (:`then`
              (`self.SetGateSettings` _returnvalue_5))))
        (:`NewEnumerator1`
          (bind _returnvalue_6 (`|GetDataTableRow` "/Game/ALS/DataTables/DT_KatanaGate.DT_KatanaGate" "KatanaCrouch")
            (:`then`
              (`self.SetGateSettings` _returnvalue_6))))))
    (:`NewEnumerator3`
      (switch `/Game/ALS/Enums/E_Weapons` (`self.EquipedWeapon`)
        (:`NewEnumerator1`
          (bind _returnvalue_7 (`|GetDataTableRow` "/Game/ALS/DataTables/DT_KatanaGate.DT_KatanaGate" "KatanaCrouchJog")
            (:`then`
              (`self.SetGateSettings` _returnvalue_7))))))))

(fn `UserConstructionScript`)
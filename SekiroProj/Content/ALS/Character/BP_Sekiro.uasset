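; BP_Sekiro is a playable character Blueprint in an ALS folder, handling movement, camera look and weapon selection through Enhanced Input.
; On BeginPlay it adds the IMC_ALS mapping context and links the ABL_Layers animation class layers to the mesh.
; Movement derives both axes from control-rotation right vectors, while look drives controller yaw and pitch.
; Weapon switching only sets the EquipedWeapon enum and prints it.
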(event `self.ReceiveBeginPlay`
  (bind _asplayer_controller (cast `PlayerController` (`self.GetController`)))
  (message `EnhancedInputSubsystemInterface.AddMappingContext` (pcsubsystem `EnhancedInputLocalPlayerSubsystem` _asplayer_controller) "/Game/ALS/Inputs/IMC_ALS.IMC_ALS" 0 (struct))
  (`SkeletalMeshComponent.LinkAnimClassLayers` (`self.Mesh`) "/Game/ALS/AnimationBlueprints/ABL_Layers.ABL_Layers_C"))

(event `EnhancedInput|/Game/ALS/Inputs/InputActions/IA_Move`
  (params (ActionValue :type "Vector2D Structure") (ElapsedSeconds :type "Float (double-precision)") (TriggeredSeconds :type "Float (double-precision)") (InputAction :type "InputAction Object Reference" :default "/Game/ALS/Inputs/InputActions/IA_Move.IA_Move"))
  (bind (_x _y) (`KismetMathLibrary.BreakVector2D` ActionValue))
  (bind (_returnvalue_roll _returnvalue_pitch _returnvalue_yaw) (`KismetMathLibrary.BreakRotator` (`self.GetControlRotation`)))
  (bind (_returnvalue_roll_2 _returnvalue_pitch_2 _returnvalue_yaw_2) (`KismetMathLibrary.BreakRotator` (`self.GetControlRotation`)))
  (:`Triggered`
    (`self.AddMovementInput` (`KismetMathLibrary.GetRightVector` (`KismetMathLibrary.MakeRotator` _returnvalue_roll_2 0.0 _returnvalue_yaw_2)) _x)
    (`self.AddMovementInput` (`KismetMathLibrary.GetRightVector` (`KismetMathLibrary.MakeRotator` 0.0 0.0 _returnvalue_yaw)) _y)))

(event `EnhancedInput|/Game/ALS/Inputs/InputActions/IA_Look`
  (params (ActionValue :type "Vector2D Structure") (ElapsedSeconds :type "Float (double-precision)") (TriggeredSeconds :type "Float (double-precision)") (InputAction :type "InputAction Object Reference" :default "/Game/ALS/Inputs/InputActions/IA_Look.IA_Look"))
  (bind (_x _y) (`KismetMathLibrary.BreakVector2D` ActionValue))
  (:`Triggered`
    (`self.AddControllerYawInput` _x)
    (`self.AddControllerPitchInput` _y)))

(event `EnhancedInput|/Game/ALS/Inputs/InputActions/IA_SwitchWeapon`
  (params (ActionValue :type "Float (double-precision)") (ElapsedSeconds :type "Float (double-precision)") (TriggeredSeconds :type "Float (double-precision)") (InputAction :type "InputAction Object Reference" :default "/Game/ALS/Inputs/InputActions/IA_SwitchWeapon.IA_SwitchWeapon"))
  (:`Started`
    (switch `int` (`KismetMathLibrary.FTrunc` ActionValue)
      (:`1`
        (set `self.EquipedWeapon` "NewEnumerator0"))
      (:`2`
        (set `self.EquipedWeapon` "NewEnumerator1"))
      (:`3`
        (set `self.EquipedWeapon` "NewEnumerator2")))
    (`KismetSystemLibrary.PrintString` (`|GetEnumeratorNameAsString` (`self.EquipedWeapon`)))))

(fn `UserConstructionScript`)